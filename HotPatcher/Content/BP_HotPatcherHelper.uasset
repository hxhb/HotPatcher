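; Blueprint helper for HotPatcher that works out which assets changed between two Git commits and builds cook commands for patch paks.
; Snapshots project asset dependencies to JSON, and reloads saved snapshots from Saved/HotPatcher, named by begin commit hash for diffs.
; Git diffs yield changed content and its dependencies, which are compared against the snapshot to find new dependencies.
; ExportPakList merges both sets into platform-specific cook commands.
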(fn `DiffNewAssetDependencies`
  (params (InBeginCommitHash :type String) (InEndCommitHash :type String))
  (returns (ReturnValue :type "AssetDependenciesInfo Structure") (rResault :type Boolean))
  (bind (_outcontentdiffinfo _outdiffassetdependencies _returnvalue) (`FlibPatchParserHelper.DiffCommitVersionAsAssetDependencies` (`FlibSourceControlHelper.GetGitBinary`) (`KismetSystemLibrary.GetProjectDirectory`) InBeginCommitHash InEndCommitHash))
  (if _returnvalue
    (bind _outstring (`FlibAssetManageHelper.LoadFileToString` (`BlueprintPathsLibrary.Combine` (`|MakeArray` (`KismetSystemLibrary.GetProjectSavedDirectory`) "HotPatcher" (`KismetStringLibrary.Concat_StrStr` InBeginCommitHash ".json")))))
    (bind (_outassetdependencies _returnvalue_2) (`FlibAssetManageHelper.DeserializeAssetDependencies` _outstring))
    (if _returnvalue_2
      (bind _returnvalue_3 (`FlibAssetManageHelper.ParserNewDependencysInfo` _outdiffassetdependencies _outassetdependencies))
      (return _returnvalue_3 true))))

(fn `DiffPatchVersionBP`
  (params (InBeginCommitHash :type String) (InEndCommitHash :type String))
  (returns (FinalAsset1 :type "AssetDependenciesInfo Structure"))
  (locals (FinalAsset :type "AssetDependenciesInfo Structure"))
  (bind (_outabspathresault _outerrormessages _returnvalue) (`FlibPatchParserHelper.DiffCommitVersion` (`FlibSourceControlHelper.GetGitBinary`) (`KismetSystemLibrary.GetProjectDirectory`) InBeginCommitHash InEndCommitHash))
  (if _returnvalue
    (bind _outresault (`FlibPatchParserHelper.GetAllEnabledModuleBaseDir`))
    (bind _outpathlist (`FlibPatchParserHelper.FilterContentPathInArray` _outresault _outabspathresault))
    (bind _outrelativepath (`FlibAssetManageHelper.ConvAssetPathListFromAbsToRelative` (`KismetSystemLibrary.GetProjectDirectory`) _outpathlist))
    (for _array_element _outrelativepath
      (set `local.FinalAsset` (`FlibAssetManageHelper.CombineAssetDependencies` (`local.FinalAsset`) (`FlibAssetManageHelper.GetAssetDependencies` _array_element))))
    (return (`local.FinalAsset`))))

(fn `ExportCurrentAssetDependency`
  (params (InFile :type String))
  (returns (ReturnValue :type Boolean))
  (bind _outalldependencies (`FlibAssetManageHelper.ExportProjectAssetDependencies` (`KismetSystemLibrary.GetProjectDirectory`)))
  (bind (_outjsonstr _returnvalue) (`FlibAssetManageHelper.SerializeAssetDependenciesToJson` _outalldependencies))
  (if _returnvalue
    (bind _returnvalue_2 (`FlibAssetManageHelper.SaveStringToFile` InFile _outjsonstr))
    (return _returnvalue_2)))

(fn `ExportPakList`
  (params (InBeginCommitHash :type String) (InEndCommitHash :type String) (InPlatformName :type String) (InCookParams :type "Array of String (by ref)"))
  (returns (OutCookCommand :type "Array of String") (ReturnValue :type Boolean))
  (bind (_outcontentdiffinfo _outdiffassetdependencies _returnvalue) (`FlibPatchParserHelper.DiffCommitVersionAsAssetDependencies` (`FlibSourceControlHelper.GetGitBinary`) (`KismetSystemLibrary.GetProjectDirectory`) InBeginCommitHash InEndCommitHash))
  (if _returnvalue
    (bind (_outassetdependencies _returnvalue_2) (`self.LoadAssetDependenciesIndo` (`KismetStringLibrary.Concat_StrStr` InBeginCommitHash ".json") (`local.__WorldContext`)))
    (if _returnvalue_2
      (bind _returnvalue_3 (`FlibAssetManageHelper.ParserNewDependencysInfo` _outdiffassetdependencies _outassetdependencies))
      (bind (_outcookcommand _returnvalue_4) (`FlibAssetManageHelper.GetCookCommandFromAssetDependencies` (`KismetSystemLibrary.GetProjectDirectory`) InPlatformName (`FlibAssetManageHelper.CombineAssetDependencies` _returnvalue_3 _outcontentdiffinfo) InCookParams))
      (return _outcookcommand _returnvalue_4))))

(fn `LoadAssetDependenciesIndo`
  (params (FileName :type String))
  (returns (OutAssetDependencies :type "AssetDependenciesInfo Structure") (ReturnValue :type Boolean))
  (bind (_outstring _returnvalue) (`FlibAssetManageHelper.LoadFileToString` (`BlueprintPathsLibrary.Combine` (`|MakeArray` (`KismetSystemLibrary.GetProjectSavedDirectory`) "HotPatcher" FileName))))
  (if _returnvalue
    (bind (_outassetdependencies _returnvalue_2) (`FlibAssetManageHelper.DeserializeAssetDependencies` _outstring))
    (return _outassetdependencies _returnvalue_2)))